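; BP_ArhiTeach_Background is a configurable backdrop actor built from six mesh components named by axis direction, apparently forming a box around the scene.
; Its construction script applies a shared height offset from HorizonLine, yaw and scale to all six meshes.
; It also pushes brightness, contrast, desaturation and emissive values into their material parameters.
; The event graph has no active runtime logic.
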(fn `UserConstructionScript`
  (bind _sm_pz (`self.SM_pz`))
  (bind _scalexy (`self.ScaleXY`))
  (`SceneComponent.K2_SetRelativeLocationAndRotation` _sm_pz (`KismetMathLibrary.MakeVector` 0.0 0.0 (- (`self.HorizonLine`) 24000.0)) (`KismetMathLibrary.MakeRotator` 0.0 0.0 (`self.Angle`)) false false)
  (`SceneComponent.K2_SetRelativeLocationAndRotation` (`self.SM_px`) (`KismetMathLibrary.MakeVector` 0.0 0.0 (- (`self.HorizonLine`) 24000.0)) (`KismetMathLibrary.MakeRotator` 0.0 0.0 (`self.Angle`)) false false)
  (`SceneComponent.K2_SetRelativeLocationAndRotation` (`self.SM_nz`) (`KismetMathLibrary.MakeVector` 0.0 0.0 (- (`self.HorizonLine`) 24000.0)) (`KismetMathLibrary.MakeRotator` 0.0 0.0 (`self.Angle`)) false false)
  (`SceneComponent.K2_SetRelativeLocationAndRotation` (`self.SM_ny`) (`KismetMathLibrary.MakeVector` 0.0 0.0 (- (`self.HorizonLine`) 24000.0)) (`KismetMathLibrary.MakeRotator` 0.0 0.0 (`self.Angle`)) false false)
  (`SceneComponent.K2_SetRelativeLocationAndRotation` (`self.SM_py`) (`KismetMathLibrary.MakeVector` 0.0 0.0 (- (`self.HorizonLine`) 24000.0)) (`KismetMathLibrary.MakeRotator` 0.0 0.0 (`self.Angle`)) false false)
  (`SceneComponent.K2_SetRelativeLocationAndRotation` (`self.SM_nx`) (`KismetMathLibrary.MakeVector` 0.0 0.0 (- (`self.HorizonLine`) 24000.0)) (`KismetMathLibrary.MakeRotator` 0.0 0.0 (`self.Angle`)) false false)
  (`SceneComponent.SetRelativeScale3D` _sm_pz (`KismetMathLibrary.MakeVector` _scalexy _scalexy (`self.ScaleZ`)))
  (`SceneComponent.SetRelativeScale3D` (`self.SM_px`) (`KismetMathLibrary.MakeVector` _scalexy _scalexy (`self.ScaleZ`)))
  (`SceneComponent.SetRelativeScale3D` (`self.SM_nz`) (`KismetMathLibrary.MakeVector` _scalexy _scalexy (`self.ScaleZ`)))
  (`SceneComponent.SetRelativeScale3D` (`self.SM_ny`) (`KismetMathLibrary.MakeVector` _scalexy _scalexy (`self.ScaleZ`)))
  (`SceneComponent.SetRelativeScale3D` (`self.SM_py`) (`KismetMathLibrary.MakeVector` _scalexy _scalexy (`self.ScaleZ`)))
  (`SceneComponent.SetRelativeScale3D` (`self.SM_nx`) (`KismetMathLibrary.MakeVector` _scalexy _scalexy (`self.ScaleZ`)))
  (`MeshComponent.SetScalarParameterValueOnMaterials` _sm_pz "Brightness" (`self.Brightness`))
  (`MeshComponent.SetScalarParameterValueOnMaterials` (`self.SM_px`) "Brightness" (`self.Brightness`))
  (`MeshComponent.SetScalarParameterValueOnMaterials` (`self.SM_nz`) "Brightness" (`self.Brightness`))
  (`MeshComponent.SetScalarParameterValueOnMaterials` (`self.SM_ny`) "Brightness" (`self.Brightness`))
  (`MeshComponent.SetScalarParameterValueOnMaterials` (`self.SM_py`) "Brightness" (`self.Brightness`))
  (`MeshComponent.SetScalarParameterValueOnMaterials` (`self.SM_nx`) "Brightness" (`self.Brightness`))
  (`MeshComponent.SetScalarParameterValueOnMaterials` _sm_pz "Contrast" (`self.Contrast`))
  (`MeshComponent.SetScalarParameterValueOnMaterials` (`self.SM_px`) "Contrast" (`self.Contrast`))
  (`MeshComponent.SetScalarParameterValueOnMaterials` (`self.SM_nz`) "Contrast" (`self.Contrast`))
  (`MeshComponent.SetScalarParameterValueOnMaterials` (`self.SM_ny`) "Contrast" (`self.Contrast`))
  (`MeshComponent.SetScalarParameterValueOnMaterials` (`self.SM_py`) "Contrast" (`self.Contrast`))
  (`MeshComponent.SetScalarParameterValueOnMaterials` (`self.SM_nx`) "Contrast" (`self.Contrast`))
  (`MeshComponent.SetScalarParameterValueOnMaterials` _sm_pz "Desaturate" (`self.Desaturate`))
  (`MeshComponent.SetScalarParameterValueOnMaterials` (`self.SM_px`) "Desaturate" (`self.Desaturate`))
  (`MeshComponent.SetScalarParameterValueOnMaterials` (`self.SM_nz`) "Desaturate" (`self.Desaturate`))
  (`MeshComponent.SetScalarParameterValueOnMaterials` (`self.SM_ny`) "Desaturate" (`self.Desaturate`))
  (`MeshComponent.SetScalarParameterValueOnMaterials` (`self.SM_py`) "Desaturate" (`self.Desaturate`))
  (`MeshComponent.SetScalarParameterValueOnMaterials` (`self.SM_nx`) "Desaturate" (`self.Desaturate`))
  (`MeshComponent.SetScalarParameterValueOnMaterials` _sm_pz "Emissive" (`self.Emissive`))
  (`MeshComponent.SetScalarParameterValueOnMaterials` (`self.SM_px`) "Emissive" (`self.Emissive`))
  (`MeshComponent.SetScalarParameterValueOnMaterials` (`self.SM_nz`) "Emissive" (`self.Emissive`))
  (`MeshComponent.SetScalarParameterValueOnMaterials` (`self.SM_ny`) "Emissive" (`self.Emissive`))
  (`MeshComponent.SetScalarParameterValueOnMaterials` (`self.SM_py`) "Emissive" (`self.Emissive`))
  (`MeshComponent.SetScalarParameterValueOnMaterials` (`self.SM_nx`) "Emissive" (`self.Emissive`)))